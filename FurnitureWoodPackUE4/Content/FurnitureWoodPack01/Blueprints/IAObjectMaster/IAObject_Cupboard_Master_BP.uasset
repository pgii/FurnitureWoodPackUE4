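; Master Blueprint for interactive cupboard furniture that swings the selected door open or closed through a quarter turn.
; On Interaction it takes the door from the level's IAObject_Controller ActiveComponent and sets BreakInteraction until the move finishes.
; Swing direction follows whether yaw is near zero and whether negative Y scale marks a mirrored door.
; The OpenMovement timeline lerps relative rotation from the starting rotator.
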(event `self.ReceiveBeginPlay`
  (bind _outactors (`GameplayStatics.GetAllActorsOfClass` "/Game/FurnitureWoodPack01/Blueprints/IAObject_Controller.IAObject_Controller_C"))
  (set `self.IAObjectController` (`|GetArrayItem` _outactors)))

(event `self.Interaction`
  (if (not (`self.isMoving`))
    (set `/Game/FurnitureWoodPack01/Blueprints/IAObject_Controller.BreakInteraction` true (`self.IAObjectController`))
    (`self.PrepareMovement`)))

(event `PrepareMovement`
  (bind _relativerotation (`SceneComponent.RelativeRotation` (`/Game/FurnitureWoodPack01/Blueprints/IAObject_Controller.ActiveComponent` (`self.IAObjectController`))))
  (set `self.isMoving` true)
  (set `self.DoorOriginalRotator` _relativerotation)
  (if (`KismetMathLibrary.NearlyEqual_FloatFloat` (.yaw _relativerotation) 0.0 1.0)
    (if (== (.y (`SceneComponent.RelativeScale3D` (`/Game/FurnitureWoodPack01/Blueprints/IAObject_Controller.ActiveComponent` (`self.IAObjectController`)))) -1.0)
      (set `self.DoorRotationY` -90.0)
      (else
        (set `self.DoorRotationY` 90.0)))
    (elif (== (.y (`SceneComponent.RelativeScale3D` (`/Game/FurnitureWoodPack01/Blueprints/IAObject_Controller.ActiveComponent` (`self.IAObjectController`)))) -1.0)
      (set `self.DoorRotationY` 90.0)
      (else
        (set `self.DoorRotationY` -90.0))))
  (`self.RotateDoor`))

(event `RotateDoor`
  (bind _doororiginalrotator (`self.DoorOriginalRotator`))
  (bind (_direction _movement) (`Timeline|OpenMovement` :!via `PlayFromStart`)
    (:`Update`
      (`SceneComponent.K2_SetRelativeRotation` (`/Game/FurnitureWoodPack01/Blueprints/IAObject_Controller.ActiveComponent` (`self.IAObjectController`)) (`KismetMathLibrary.RLerp` _doororiginalrotator (`KismetMathLibrary.MakeRotator` (.roll _doororiginalrotator) (.pitch _doororiginalrotator) (+ (.yaw _doororiginalrotator) (`self.DoorRotationY`))) _movement) false false))
    (:`Finished`
      (set `self.isMoving` false)
      (set `/Game/FurnitureWoodPack01/Blueprints/IAObject_Controller.BreakInteraction` false (`self.IAObjectController`)))))

(fn `UserConstructionScript`
  (`parent.UserConstructionScript`))