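; Master Blueprint for an interactable furniture drawer that slides open and closed on Interaction.
; It moves the active component reported by the level's IAObject_Controller, choosing direction by whether its relative X is near zero and DrawerDepth's sign.
; A timeline lerps the component along relative X, while IsMoving and the controller's BreakInteraction flag stay set until it finishes.
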(event `self.ReceiveBeginPlay`
  (bind _outactors (`GameplayStatics.GetAllActorsOfClass` "/Game/FurnitureWoodPack01/Blueprints/IAObject_Controller.IAObject_Controller_C"))
  (set `self.IAObjectController` (`|GetArrayItem` _outactors)))

(event `self.Interaction`
  (if (not (`self.isMoving`))
    (set `/Game/FurnitureWoodPack01/Blueprints/IAObject_Controller.BreakInteraction` true (`self.IAObjectController`))
    (`self.MoveDrawer`)))

(event `MoveDrawer`
  (bind _relativelocation (`SceneComponent.RelativeLocation` (`/Game/FurnitureWoodPack01/Blueprints/IAObject_Controller.ActiveComponent` (`self.IAObjectController`))))
  (set `self.isMoving` true)
  (set `self.DrawerOrigin` _relativelocation)
  (if (`KismetMathLibrary.NearlyEqual_FloatFloat` (.x _relativelocation) 0.0 1.0)
    (if (< (`self.DrawerDepth`) 0.0)
      (`/Engine/EditorBlueprintResources/StandardMacros.NegateFloat` (`self.DrawerDepth`)
        (:`  `
          _)))
    (elif (not (< (`self.DrawerDepth`) 0.0))
      (`/Engine/EditorBlueprintResources/StandardMacros.NegateFloat` (`self.DrawerDepth`)
        (:`  `
          _))))
  (`self.Move`))

(event `Move`
  (bind _drawerorigin (`self.DrawerOrigin`))
  (bind (_direction _movement) (`Timeline|DrawerMovement` :!via `PlayFromStart`)
    (:`Update`
      (`SceneComponent.K2_SetRelativeLocation` (`/Game/FurnitureWoodPack01/Blueprints/IAObject_Controller.ActiveComponent` (`self.IAObjectController`)) (`KismetMathLibrary.VLerp` _drawerorigin (`KismetMathLibrary.MakeVector` (+ (.x _drawerorigin) (`self.DrawerDepth`)) (.y _drawerorigin) (.z _drawerorigin)) _movement) false false))
    (:`Finished`
      (set `self.isMoving` false)
      (set `/Game/FurnitureWoodPack01/Blueprints/IAObject_Controller.BreakInteraction` false (`self.IAObjectController`)))))

(fn `UserConstructionScript`
  (`parent.UserConstructionScript`))