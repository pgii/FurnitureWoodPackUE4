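; Master Blueprint for an interactable ceiling fan in the furniture pack.
; Each tick, while enabled, it adds a yaw rotation scaled by Speed to four blade components.
; The Interaction event toggles the fan on and off.
; Rotation is a fixed per-tick increment without delta time, so spin speed varies with frame rate.
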(event `self.ReceiveTick`
  (params (DeltaSeconds :type "Float (single-precision)"))
  (if (`self.isEnable`)
    (`SceneComponent.K2_AddRelativeRotation` (`self.Blade01`) (`KismetMathLibrary.MakeRotator` 0.0 0.0 (`self.Speed`)) false false)
    (`SceneComponent.K2_AddRelativeRotation` (`self.Blade02`) (`KismetMathLibrary.MakeRotator` 0.0 0.0 (`self.Speed`)) false false)
    (`SceneComponent.K2_AddRelativeRotation` (`self.Blade03`) (`KismetMathLibrary.MakeRotator` 0.0 0.0 (`self.Speed`)) false false)
    (`SceneComponent.K2_AddRelativeRotation` (`self.Blade04`) (`KismetMathLibrary.MakeRotator` 0.0 0.0 (`self.Speed`)) false false)))

(event `self.Interaction`
  (set `self.isEnable` (not (`self.isEnable`))))

(fn `UserConstructionScript`
  (`parent.UserConstructionScript`))