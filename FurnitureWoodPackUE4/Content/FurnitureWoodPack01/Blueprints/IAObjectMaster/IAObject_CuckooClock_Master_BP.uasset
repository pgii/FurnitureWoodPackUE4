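; Master Blueprint for an interactable cuckoo clock whose door swings open or shut while the cuckoo slides out or back in.
; On interaction, it checks the shared IAObject_Controller's active component for the door tag and blocks further interaction during movement.
; Two timelines drive door yaw and cuckoo position, inferring direction from current transforms and mirrored door scale.
; A short delay staggers them: door first when opening, cuckoo first when closing.
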(event `self.ReceiveBeginPlay`
  (bind _outactors (`GameplayStatics.GetAllActorsOfClass` "/Game/FurnitureWoodPack01/Blueprints/IAObject_Controller.IAObject_Controller_C"))
  (set `self.IAObjectController` (`|GetArrayItem` _outactors)))

(event `self.Interaction`
  (if (not (`self.isMoving`))
    (set `/Game/FurnitureWoodPack01/Blueprints/IAObject_Controller.BreakInteraction` true (`self.IAObjectController`))
    (`self.CheckInteactiveType`)))

(event `CheckInteactiveType`
  (if (`ActorComponent.ComponentHasTag` (`/Game/FurnitureWoodPack01/Blueprints/IAObject_Controller.ActiveComponent` (`self.IAObjectController`)) "IAObjectDoor")
    (`self.PrepareMovement`)))

(event `MoveCuckoo`
  (bind _relativelocation (`SceneComponent.RelativeLocation` (`self.Cuckoo`)))
  (set `self.isMoving` true)
  (set `self.DrawerOrigin` _relativelocation)
  (if (`KismetMathLibrary.NearlyEqual_FloatFloat` (.x _relativelocation) 0.0 1.0)
    (if (< (`self.DrawerDepth`) 0.0)
      (`/Engine/EditorBlueprintResources/StandardMacros.NegateFloat` (`self.DrawerDepth`)
        (:`  `
          _)))
    (elif (not (< (`self.DrawerDepth`) 0.0))
      (`/Engine/EditorBlueprintResources/StandardMacros.NegateFloat` (`self.DrawerDepth`)
        (:`  `
          _))))
  (`self.Move`))

(event `Move`
  (bind _drawerorigin (`self.DrawerOrigin`))
  (bind (_direction _movement) (`Timeline|CuckooMovement` :!via `PlayFromStart`)
    (:`Update`
      (`SceneComponent.K2_SetRelativeLocation` (`self.Cuckoo`) (`KismetMathLibrary.VLerp` _drawerorigin (`KismetMathLibrary.MakeVector` (+ (.x _drawerorigin) (`self.DrawerDepth`)) (.y _drawerorigin) (.z _drawerorigin)) _movement) false false))
    (:`Finished`
      (set `self.isMoving` false)
      (set `/Game/FurnitureWoodPack01/Blueprints/IAObject_Controller.BreakInteraction` false (`self.IAObjectController`)))))

(event `PrepareMovement`
  (bind _relativerotation (`SceneComponent.RelativeRotation` (`/Game/FurnitureWoodPack01/Blueprints/IAObject_Controller.ActiveComponent` (`self.IAObjectController`))))
  (set `self.isMoving` true)
  (set `self.DoorOriginalRotator` _relativerotation)
  (if (`KismetMathLibrary.NearlyEqual_FloatFloat` (.yaw _relativerotation) 0.0 1.0)
    (if (== (.y (`SceneComponent.RelativeScale3D` (`/Game/FurnitureWoodPack01/Blueprints/IAObject_Controller.ActiveComponent` (`self.IAObjectController`)))) -1.0)
      (set `self.DoorRotationY` -90.0)
      (else
        (set `self.DoorRotationY` 90.0)))
    (`self.RotateDoor`)
    (`KismetSystemLibrary.Delay` 0.2)
    (`self.MoveCuckoo`)
    (else
      (if (== (.y (`SceneComponent.RelativeScale3D` (`/Game/FurnitureWoodPack01/Blueprints/IAObject_Controller.ActiveComponent` (`self.IAObjectController`)))) -1.0)
        (set `self.DoorRotationY` 90.0)
        (else
          (set `self.DoorRotationY` -90.0)))
      (`self.MoveCuckoo`)
      (`KismetSystemLibrary.Delay` 0.2)
      (`self.RotateDoor`))))

(event `RotateDoor`
  (bind _doororiginalrotator (`self.DoorOriginalRotator`))
  (bind (_direction _movement) (`Timeline|TimelineRotateDoor` :!via `PlayFromStart`)
    (:`Update`
      (`SceneComponent.K2_SetRelativeRotation` (`/Game/FurnitureWoodPack01/Blueprints/IAObject_Controller.ActiveComponent` (`self.IAObjectController`)) (`KismetMathLibrary.RLerp` _doororiginalrotator (`KismetMathLibrary.MakeRotator` (.roll _doororiginalrotator) (.pitch _doororiginalrotator) (+ (.yaw _doororiginalrotator) (`self.DoorRotationY`))) _movement) false false))
    (:`Finished`
      (set `self.isMoving` false)
      (set `/Game/FurnitureWoodPack01/Blueprints/IAObject_Controller.BreakInteraction` false (`self.IAObjectController`)))))

(fn `UserConstructionScript`
  (`parent.UserConstructionScript`))