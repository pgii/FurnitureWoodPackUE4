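; Interaction controller that lets the player use tagged furniture objects, drawers and doors, and adds a HUD widget at BeginPlay.
; Each tick, a short camera-forward line trace stores the hit actor and component when the component carries an interaction tag.
; The current object clears on a miss, while the pawn moves, or when BreakInteraction is set.
; The Interaction input calls Interaction on that object through a cast to IAObject_Master_BP.
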(event `self.ReceiveBeginPlay`
  (bind _returnvalue (`|CreateWidget` "/Game/FurnitureWoodPack01/Blueprints/HUD/HUD.HUD_C"))
  (`UserWidget.AddToViewport` _returnvalue 0))

(event `self.ReceiveTick`
  (params (DeltaSeconds :type "Float (single-precision)"))
  (`self.CheckInteractionObject`))

(event `InputAction|Interaction`
  (params (Key :type "Key Structure"))
  (:`Pressed`
    (bind _asiaobject_master_bp (cast `/Game/FurnitureWoodPack01/Blueprints/IAObjectMaster/IAObject_Master_BP` (`self.CurrentInteractionObject`)))
    (`/Game/FurnitureWoodPack01/Blueprints/IAObjectMaster/IAObject_Master_BP.Interaction` _asiaobject_master_bp)))

(event `CheckInteractionObject`
  (bind _returnvalue (`GameplayStatics.GetPlayerCameraManager` 0))
  (bind _returnvalue_2 (`self.K2_GetActorLocation` _returnvalue))
  (if (`self.BreakInteraction`)
    (set `self.CurrentInteractionObject` null :!label _label)
    (elif (> (`KismetMathLibrary.VSize` (`self.GetVelocity` (`GameplayStatics.GetPlayerPawn` 0))) 0.0)
      (goto _label)
      (else
        (bind (_outhit _returnvalue_3) (`KismetSystemLibrary.LineTraceSingle` _returnvalue_2 (+ _returnvalue_2 (* (`self.GetActorForwardVector` _returnvalue) 220.0)) "TraceTypeQuery1"))
        (if _returnvalue_3
          (bind (_bblockinghit _binitialoverlap _time _distance _location _impactpoint _normal _impactnormal _physmat _hitactor _hitcomponent) (`GameplayStatics.BreakHitResult` _outhit))
          (if (or (`ActorComponent.ComponentHasTag` _hitcomponent "IAObject") (`ActorComponent.ComponentHasTag` _hitcomponent "IAObjectDrawer") (`ActorComponent.ComponentHasTag` _hitcomponent "IAObjectDoor"))
            (set `self.CurrentInteractionObject` _hitactor)
            (set `self.ActiveComponent` _hitcomponent)
            (else
              (set `self.CurrentInteractionObject` null :!label _label_2)))
          (else
            (goto _label_2)))))))

(fn `UserConstructionScript`)